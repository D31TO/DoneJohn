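; BP_Barrel is a breakable barrel that drops a coin pickup when hit through the EnemyOuch event.
; It carries enemy-style character components but destroys its movement, mesh, pawn sensing and groan components on BeginPlay, leaving a static prop.
; EnemyOuch spawns a CoinPickup at the Barrel component's location, then destroys the actor.
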(event `self.ReceiveBeginPlay`
  (`ActorComponent.K2_DestroyComponent` (`self.CharacterMovement`))
  (`ActorComponent.K2_DestroyComponent` (`self.Mesh`))
  (`ActorComponent.K2_DestroyComponent` (`self.PawnSensing`))
  (`ActorComponent.K2_DestroyComponent` (`self.Groan`)))

(event `self.EnemyOuch`
  (`|SpawnActorFromClass` "/Game/Assets/Pickups/CoinPickup.CoinPickup_C" (`KismetMathLibrary.Conv_VectorToTransform` (`SceneComponent.K2_GetComponentLocation` (`self.Barrel`))) "Undefined" "MultiplyWithRoot" null null)
  (`self.K2_DestroyActor`))

(fn `UserConstructionScript`
  (`parent.UserConstructionScript`))