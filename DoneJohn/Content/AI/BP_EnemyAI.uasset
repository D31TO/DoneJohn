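; BP_EnemyAI is a zombie enemy character that detects the player and performs a melee attack.
; Pawn sensing sets the HasSeenPlayer blackboard key on its AI controller when it sees the first-person character, and never clears it here.
; The Attack event sphere-traces a short distance forward for pawns, with debug drawing on.
; On hitting the player, it plays the attack montage and immediately calls TakeDamage on them.
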(event `self.PawnSensing.OnSeePawn`
  (params (Pawn :type "Pawn Object Reference"))
  ;[1 0.08259 0] Goto player
  (cast `/Game/FirstPerson/Blueprints/BP_FirstPersonCharacter` Pawn)
  (`BlackboardComponent.SetValueAsBool` (`AIBlueprintHelperLibrary.GetBlackboard` (`AIBlueprintHelperLibrary.GetAIController` self)) "HasSeenPlayer" true))

(event `Attack`
  (bind _returnvalue (`self.K2_GetActorLocation`))
  ;[1 0 0] Attack
  (bind (_outhit _returnvalue_2) (`KismetSystemLibrary.SphereTraceSingleForObjects` :`Start` _returnvalue :`End` (+ _returnvalue (* (`KismetMathLibrary.GetForwardVector` (`self.K2_GetActorRotation`)) 250.0)) :`Radius` 50.0 :`ObjectTypes` (`|MakeArray` "ObjectTypeQuery3" :!type "EObjectTypeQuery Enum") :`DrawDebugType` "ForDuration"))
  (if _returnvalue_2
    (bind _asbp_first_person_character (cast `/Game/FirstPerson/Blueprints/BP_FirstPersonCharacter` (`.HitActor` (`GameplayStatics.BreakHitResult` _outhit))))
    (`self.PlayAnimMontage` "/Game/Mixamo/Zombie/Animations/Zombie_Attack_Montage.Zombie_Attack_Montage")
    (`/Game/FirstPerson/Blueprints/BP_FirstPersonCharacter.TakeDamage` _asbp_first_person_character)))

(fn `UserConstructionScript`)